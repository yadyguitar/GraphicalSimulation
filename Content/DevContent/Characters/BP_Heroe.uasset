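; BP_Heroe is a first-person player character with movement, look, jumping, a run toggle and shooting.
; On BeginPlay it spawns and attaches a BP_Rifle, which it fires from the camera, gated by ammo and a Delay-based fire rate.
; An empty magazine shows a BP_Info widget until reload refills it.
; Any actor overlap grants a temporary triple jump, timed by a frame countdown in Tick.
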(event `self.ReceiveBeginPlay`
  (bind _equippedgun (`self.EquippedGun`))
  (bind _returnvalue (`|SpawnActorFromClass` "/Game/Objects/Guns/machinegun/BP_Rifle.BP_Rifle_C" (`KismetMathLibrary.MakeTransform` (0.0 0.0 0.0)) "Undefined" "OverrideRootScale" null null))
  (bind _output_get (set `self.EquippedGun` _returnvalue))
  (`self.K2_AttachToComponent` _output_get (`self.PersonalGunLocation`) "None" "KeepRelative" "KeepRelative" "KeepRelative" true)
  (set `/Game/Objects/Guns/BP_BaseGun.RemainBullets` (`/Game/Objects/Guns/BP_BaseGun.MagazineSize` _equippedgun) _equippedgun))

(event `InputAxis|M_Forward`
  (params (AxisValue :type "Float (single-precision)"))
  (`self.AddMovementInput` (`self.GetActorForwardVector`) AxisValue))

(event `InputAxis|M_Right`
  (params (AxisValue :type "Float (single-precision)"))
  (`self.AddMovementInput` (`self.GetActorRightVector`) AxisValue))

(event `InputAxis|M_Yaw`
  (params (AxisValue :type "Float (single-precision)"))
  (`self.AddControllerYawInput` AxisValue))

(event `InputAxis|M_Pitch`
  (params (AxisValue :type "Float (single-precision)"))
  (`self.AddControllerPitchInput` (* AxisValue -1.0)))

(event `InputAction|A_jump`
  (params (Key :type "Key Structure"))
  (:`Pressed`
    (`self.Jump`))
  (:`Released`
    (`self.StopJumping`)))

(event `self.ReceiveActorBeginOverlap`
  (params (OtherActor :type "Actor Object Reference"))
  (set `self.JumpMaxCount` 3)
  (set `self.JumpTimer` 180))

(event `self.ReceiveTick`
  (params (DeltaSeconds :type "Float (single-precision)"))
  (if (> (`self.JumpTimer`) 0)
    (bind _output_get (set `self.JumpTimer` (- (`self.JumpTimer`) 1)))
    (if (<= _output_get 0)
      (set `self.JumpMaxCount` 1))))

(event `InputAction|A_Run`
  (params (Key :type "Key Structure"))
  (bind _charactermovement (`self.CharacterMovement`))
  (:`Pressed`
    (if (`self.Run`)
      (set `self.Run` false)
      (set `CharacterMovementComponent.MaxWalkSpeed` 600.0 _charactermovement)
      (else
        (set `self.Run` true)
        (set `CharacterMovementComponent.MaxWalkSpeed` 1000.0 _charactermovement)))))

(event `InputAxis|M_Shoot`
  (params (AxisValue :type "Float (single-precision)"))
  (bind _returnvalue (`KismetMathLibrary.NearlyEqual_FloatFloat` AxisValue 1.0))
  (bind _equippedgun (`self.EquippedGun`))
  (bind _fpscamera (`self.FPSCamera`))
  (bind _returnvalue_2 (`SceneComponent.K2_GetComponentLocation` _fpscamera))
  (if (and (> (`/Game/Objects/Guns/BP_BaseGun.RemainBullets` (`self.EquippedGun`)) 0) _returnvalue)
    (if (and _returnvalue (`self.FireRateCheck`))
      (`/Game/Objects/Guns/BP_BaseGun.Shoot` (`self.EquippedGun`) _returnvalue_2 (+ _returnvalue_2 (* (`SceneComponent.GetForwardVector` _fpscamera) (`/Game/Objects/Guns/BP_BaseGun.BulletDistance` (`self.EquippedGun`)))))
      (set `/Game/Objects/Guns/BP_BaseGun.RemainBullets` (- (`/Game/Objects/Guns/BP_BaseGun.RemainBullets` _equippedgun) 1) _equippedgun)
      (if (> (`/Game/Objects/Guns/BP_BaseGun.RemainBullets` (`self.EquippedGun`)) 0)
        (set `self.FireRateCheck` false)
        (`KismetSystemLibrary.Delay` (`/Game/Objects/Guns/BP_BaseGun.FireRate` (`self.EquippedGun`)))
        (set `self.FireRateCheck` true)
        (else
          ;[1 1 1] Muestra widget en pantalla
          (bind _returnvalue_3 (`|CreateWidget` "/Game/Widgets/BP_Info.BP_Info_C"))
          (bind _output_get (set `self.BP_Info` _returnvalue_3))
          (`UserWidget.AddToViewport` _output_get 0)
          (set `self.FireRateCheck` false)
          (`KismetSystemLibrary.Delay` (`/Game/Objects/Guns/BP_BaseGun.FireRate` (`self.EquippedGun`)))
          (set `self.FireRateCheck` true))))))

(event `InputAction|A_Reload`
  (params (Key :type "Key Structure"))
  (bind _equippedgun (`self.EquippedGun`))
  (:`Pressed`
    (set `/Game/Objects/Guns/BP_BaseGun.RemainBullets` (`/Game/Objects/Guns/BP_BaseGun.MagazineSize` _equippedgun) _equippedgun)
    (if (`Widget.IsInViewport` (`self.BP_Info`))
      ;[1 1 1] Borra widget de pantalla
      (`Widget.RemoveFromParent` (`self.BP_Info`)))))

(fn `UserConstructionScript`
  (set `self.JumpMaxCount` 1)
  (set `self.JumpMaxHoldTime` 0.0)
  (set `self.Run` false))